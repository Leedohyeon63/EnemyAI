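; Base enemy Blueprint that provides back-and-forth patrol movement and state-based walk speed.
; The Patrol event uses AIMoveTo toward one of two target actors, chosen by the Reverce flag, which flips when a move succeeds.
; SetSpeed maps a movement state to the CharacterMovement max walk speed and returns it.
; BeginPlay is empty, and nothing in this file calls Patrol or SetSpeed.
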(event Custom|Patrol
  (if (Variables|Default|Getreverce)
    (AI|AIMoveTo self (Transformation|GetActorLocation (Variables|Default|Gettarget1)) 0 5.0 false
      (:OnSuccess
        (Variables|Default|Setreverce false)))
    (else
      (AI|AIMoveTo self (Transformation|GetActorLocation (Variables|Default|Gettarget2)) 0 5.0 false
        (:OnSuccess
          (Variables|Default|Setreverce true))))))

(event EventBeginPlay)

(fn ConstructionScript)

(fn SetSpeed
  (params (State :type E_Speed%20Enum :default "NewEnumerator0"))
  (bind _output_get (Variables|/Script/Engine.CharacterMovementComponent|SetMaxWalkSpeed (Variables|Character|GetCharacterMovement) (Utilities|Select :Index State :NewEnumerator0 0.0 :NewEnumerator1 1e+02 :NewEnumerator2 3e+02 :NewEnumerator3 5e+02)))
  (return _output_get))